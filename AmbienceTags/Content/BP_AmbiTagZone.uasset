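; BP_AmbiTagZone is a placeable zone that adds its contributor gameplay tags to the AmbiTag subsystem while the player pawn is inside.
; Begin and end overlap events add or remove the tags through TagUpdate, with a delayed check after BeginPlay catching a player who starts inside.
; The construction script activates and shows the box, sphere or capsule chosen by ZoneType, deactivates the others, and uses Debug for in-game visibility.
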(event Custom|DelayedCollisionCheck
  ;[1 1 1] Use this BP as a default way of adding gameplay tags to the ambitag subsystem
  ;;[1 1 1] Add tag if the player is in the box on event start
  (if (Utilities|Array|ContainsItem (Collision|GetOverlappingActors 0 :!class /Script/Engine.Actor) (Game|Player|GetPlayerPawn 0))
    (CallFunction|TagUpdate true)))

(event EventBeginPlay
  ;[1 1 1] Use this BP as a default way of adding gameplay tags to the ambitag subsystem
  ;;[1 1 1] Delayed callback to check if player is in collision box
  (Utilities|Time|SetTimerbyEvent (EventDispatchers|CreateEvent :!event Custom|DelayedCollisionCheck) 1.0))

(event Collision|EventActorBeginOverlap
  (params (OtherActor :type Actor%20Object%20Reference))
  ;[1 1 1] Use this BP as a default way of adding gameplay tags to the ambitag subsystem
  ;;[1 1 1] Add tags when player enters zone, remove when they leave
  (if (== OtherActor (Game|Player|GetPlayerPawn 0))
    (CallFunction|TagUpdate true)))

(event Collision|EventActorEndOverlap
  (params (OtherActor :type Actor%20Object%20Reference))
  ;[1 1 1] Use this BP as a default way of adding gameplay tags to the ambitag subsystem
  ;;[1 1 1] Add tags when player enters zone, remove when they leave
  (if (== (Game|Player|GetPlayerPawn 0) OtherActor)
    (CallFunction|TagUpdate false)))

(fn ConstructionScript
  (CallFunction|Activate (Variables|Default|GetZone%20Type))
  (Development|SetHiddeninGame (Variables|Default|GetCoollisionComp) (not (Variables|Default|GetDebug)) false))

(fn TagUpdate
  (params (Add :type Boolean))
  (bind _returnvalue (Subsystems|GetAmbiTagSubsystem))
  (bind _contributor_tags (Variables|Default|GetContributor%20Tags))
  (if Add
    (Class|AmbiTagSubsystem|AddAmbiTags _returnvalue _contributor_tags)
    (else
      (Class|AmbiTagSubsystem|RemoveAmbiTags _returnvalue _contributor_tags))))

(fn Activate
  (params (Zone%20Type :type EAmbiTagZoneType%20Enum :default "Box"))
  (bind _capsule (Variables|Default|GetCapsule))
  (bind _sphere (Variables|Default|GetSphere))
  (bind _box (Variables|Default|GetBox))
  (bind _returnvalue (Utilities|Select :Index Zone%20Type :Box _box :Sphere _sphere :Capsule _capsule))
  (bind _output_get (LocalVariables|SetCollisionComps (Utilities|Array|MakeArray _sphere _box _capsule)))
  (Components|Activation|Activate _returnvalue false)
  (Rendering|SetVisibility _returnvalue true false)
  (Utilities|Array|RemoveItem _output_get _returnvalue)
  (Variables|Default|SetCoollisionComp _returnvalue)
  (for _array_element (LocalVariables|GetCollisionComps)
    (Components|Activation|Deactivate _array_element)
    (Rendering|SetVisibility _array_element false false)))